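; Bullet projectile actor that fires toward the player camera with random sideways and downward aim offsets, for bullet-time effects.
; BeginPlay fires it with a 15-second lifespan, a gunshot pitched by global time dilation and an attached BulletTime sound at zero volume.
; Fire spawns a muzzle flash, resets position and sets velocity and rotation from separately randomized aim points; R refires.
; Tick adds random roll spin.
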(event `self.ReceiveBeginPlay`
  ;[1 1 1] EventBeginPlay
  (`|ExecutionSequence`
    (:`then_0`
      ;[1 1 1] Bullet spawn settings
      (`self.EnableInput` (`GameplayStatics.GetPlayerController` 0))
      (set `self.InitPos` (`self.K2_GetActorLocation`))
      (`self.Fire`)
      (`self.SetLifeSpan` 15.0))
    (:`then_1`
      ;[1 1 1] Trigger sounds
      (`GameplayStatics.SpawnSoundAtLocation` "/Game/Audio/gunshot.Gunshot" (`self.InitPos`) (struct) (`KismetMathLibrary.RandomFloatInRange` 0.8 0.9) (`KismetMathLibrary.FClamp` (* (`GameplayStatics.GetGlobalTimeDilation`) 1.0) 0.1 1.0) 0.0 "/Game/Audio/Gunshot_Attenuation.Gunshot_Attenuation"))
    (:`then_2`
      (`GameplayStatics.SpawnSoundAttached` "/Game/Audio/Bullet-Time.Bullet-Time" (`self.Bullet`) "None" (0.0 0.0 0.0) (struct) "KeepRelativeOffset" true 0.0 0.0 0.0 "/Game/Audio/Attenuation_Setting_Bullet.Attenuation_Setting_Bullet" "/Game/Audio/Concurrency_Seting_Bullet.Concurrency_Seting_Bullet"))))

(event `Key|R`
  (params (Key :type "Key Structure" :default "AnyKey"))
  (:`Pressed`
    (`self.Fire`)))

(event `Fire`
  (bind (_returnvalue_x _returnvalue_y _returnvalue_z) (`KismetMathLibrary.BreakVector` (`self.K2_GetActorLocation` (`GameplayStatics.GetPlayerCameraManager` 0))))
  (bind _returnvalue (`KismetMathLibrary.MakeVector` (+ (.x (`self.InitPos`)) -30.0) (.y (`self.InitPos`)) (.z (`self.InitPos`))))
  (bind _returnvalue_2 (`KismetMathLibrary.Normal` (- (- (`self.K2_GetActorLocation` (`GameplayStatics.GetPlayerCameraManager` 0)) (`KismetMathLibrary.MakeVector` 0.0 (`KismetMathLibrary.RandomFloatInRange` -75.0 75.0) (`KismetMathLibrary.RandomFloatInRange` 0.0 (* _returnvalue_z 0.67)))) (`self.K2_GetActorLocation`))))
  ;[1 1 1] Fire bullet
  (`GameplayStatics.SpawnEmitterAtLocation` "/Game/MyWork/Muzzle.Muzzle" _returnvalue (struct)) ; Muzzle flash
  (`self.K2_SetActorLocation` _returnvalue)
  ;[1 1 1] Calculate target
  (set `MovementComponent.Velocity` (* _returnvalue_2 100.0) (`self.ProjectileMovement`))
  (`SceneComponent.K2_SetWorldRotation` (`self.Root`) (`KismetMathLibrary.Conv_VectorToRotator` _returnvalue_2) false false))

(event `self.ReceiveTick`
  (params (DeltaSeconds :type "Float (single-precision)"))
  ;[1 1 1] Rotation of bullets
  (`self.K2_AddActorLocalRotation` (`KismetMathLibrary.MakeRotator` (`KismetMathLibrary.RandomFloatInRange` 0.25 3.0))))

(fn `UserConstructionScript`)