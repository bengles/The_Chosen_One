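; Shooter actor that fires BP_Bullet actors in waves from an offset to its position, matching its rotation.
; StartWave starts a looping spawn timer at a random interval, picked once, whose upper limit shrinks as bullets per wave grow.
; When the quota is reached, SpawnBullet clears the timer, waits, resets the count, enlarges the quota and increments Wave.
; Nothing in this graph calls StartWave or restarts the timer.
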(event `Start Wave`
  ;[1 1 1] Bullet spawn settings
  (bind _returnvalue (`KismetSystemLibrary.K2_SetTimerDelegate` (delegate `Spawn Bullet`) (`KismetMathLibrary.RandomFloatInRange` 0.0 (/ 5.0 (`KismetMathLibrary.Conv_IntToDouble` (`self.BulletsPerWave`)))) true)) ; Bullet spawn timer
)

(event `Spawn Bullet`
  ;[1 1 1] Bullet spawn settings
  (set `self.TotalShotsFired` (+ (`self.TotalShotsFired`) 1))
  (if (>= (`self.Counter`) (`self.BulletsPerWave`))
    (`KismetSystemLibrary.K2_ClearAndInvalidateTimerHandle` (stale `Start Wave` _returnvalue))
    (`KismetSystemLibrary.Delay` 10.0)
    (set `self.Counter` 0)
    (set `self.BulletsPerWave` (+ (`self.BulletsPerWave`) 3))
    (`/Engine/EditorBlueprintResources/StandardMacros.IncrementInt` (`self.Wave`))
    (else
      (set `self.Counter` (+ (`self.Counter`) 1)) ; Increase number of shots fired then spawn bullet
      (`|SpawnActorFromClass` "/Game/MyWork/Blueprints/BP_Bullet.BP_Bullet_C" (`KismetMathLibrary.MakeTransform` (+ (`self.K2_GetActorLocation`) (-35.0 -30.0 150.0)) (.rotation (`self.GetTransform`)) (0.01 0.01 0.01)) "AlwaysSpawn" "OverrideRootScale"))))

(fn `UserConstructionScript`)