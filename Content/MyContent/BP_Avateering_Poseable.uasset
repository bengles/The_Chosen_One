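; Kinect avateering Blueprint that drives a poseable mesh avatar from the body tracked at the center of the sensor's view.
; Each tick it feeds the centered body to the Kinect poseable mesh, with smoothing set at BeginPlay.
; It then moves the mesh using the rotated head bone position and a fixed offset to align the head with the camera.
; Capsule hits from BP_projectile only print a debug message.
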(event `self.ReceiveBeginPlay`
  ;[1 1 1] Configure Kinect Poseable Mesh smoothing field
  (set `KinectPoseableMeshComponent.IsSmoothing` (`self.Smoothing`) (`self.KinectPoseableMesh`)))

(event `self.ReceiveTick`
  (params (DeltaSeconds :type "Float (single-precision)"))
  ;[1 1 1] Update the Kinect Poseable Mesh to pull data from current centered body
  (bind (_centeredbody _istracked) (`KinectInterfaceComponent.GetCenteredBody` (`self.KinectInterface`)))
  (if _istracked
    (set `KinectPoseableMeshComponent.TargetBody` _centeredbody (`self.KinectPoseableMesh`))
    (bind _returnvalue (`PoseableMeshComponent.GetBoneLocationByName` (`self.KinectPoseableMesh`) "head" "ComponentSpace"))
    (`SceneComponent.K2_SetWorldLocation` (`self.KinectPoseableMesh`) (- (- (`SceneComponent.K2_GetComponentLocation` (`self.Camera`)) (`KismetMathLibrary.GreaterGreater_VectorRotator` _returnvalue (struct :`Yaw` 90.0))) (0.0 13.0 5.0)) false false)))

(event `self.KinectPoseableMesh.OnComponentHit`
  (params (HitComponent :type "PrimitiveComponent Object Reference") (OtherActor :type "Actor Object Reference") (OtherComp :type "PrimitiveComponent Object Reference") (NormalImpulse :type "Vector Structure") (Hit :type "HitResult Structure (by ref)")))

(event `self.CapsuleComponent.OnComponentHit`
  (params (HitComponent :type "PrimitiveComponent Object Reference") (OtherActor :type "Actor Object Reference") (OtherComp :type "PrimitiveComponent Object Reference") (NormalImpulse :type "Vector Structure") (Hit :type "HitResult Structure (by ref)"))
  (if (== (`GameplayStatics.GetObjectClass` OtherActor) "/Game/MyContent/BP_projectile.BP_projectile_C")
    (`KismetSystemLibrary.PrintString` "capsule hit")))

(fn `UserConstructionScript`)