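; Projectile actor in the Avateering folder that launches itself toward the first player after a random delay of a few seconds.
; On BeginPlay it waits, then sets its ProjectileMovement velocity to a slow, fixed speed aimed slightly below the player controller's actor location.
; The aim is computed once from the controller rather than the pawn, with no homing or overlap handling.
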(event `self.ReceiveBeginPlay`
  (`KismetSystemLibrary.Delay` (`KismetMathLibrary.RandomFloatInRange` 0.0 5.0))
  (set `MovementComponent.Velocity` (* (`KismetMathLibrary.Normal` (- (- (`self.K2_GetActorLocation` (`GameplayStatics.GetPlayerController` 0)) (0.0 0.0 30.0)) (`self.K2_GetActorLocation`))) 100.0) (`self.ProjectileMovement`)))

(fn `UserConstructionScript`)