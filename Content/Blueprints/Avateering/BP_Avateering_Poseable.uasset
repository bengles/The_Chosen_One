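; Player avatar for a Kinect bullet-dodging game, driving a poseable mesh from the centered tracked body.
; Each tick offsets the mesh so its head follows the camera; R rescales it by camera height.
; Torso bullet hits fade the screen red and cost a life, other body-part overlaps do nothing, and a trigger box counts dodges.
; The GameOver widget is added at start, but its game-over and pause calls are unwired.
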(event `Reset Height`
  (bind (_relativelocation_x _relativelocation_y _relativelocation_z) (`KismetMathLibrary.BreakVector` (`SceneComponent.RelativeLocation` (`self.Camera`))))
  ;[1 1 1] Reset Height
  (bind _output_get (set `self.Scale` (/ _relativelocation_z 169.0)))
  (`SceneComponent.SetWorldScale3D` (`self.KinectPoseableMesh`) (`KismetMathLibrary.Conv_DoubleToVector` _output_get)))

(event `Key|R`
  (params (Key :type "Key Structure" :default "AnyKey"))
  ;[1 1 1] Reset Height
  (:`Pressed`
    (`self.Reset Height`)))

(event `self.ReceiveBeginPlay`
  (bind (_kinectrotation_x _kinectrotation_y _kinectrotation_z) (`KismetMathLibrary.BreakVector` (`self.KinectRotation`)))
  ;[1 1 1] Configure Kinect Poseable Mesh smoothing field
  (set `KinectPoseableMeshComponent.IsSmoothing` (`self.Smoothing`) (`self.KinectPoseableMesh`))
  (`SceneComponent.K2_SetRelativeRotation` (`self.KinectPoseableMesh`) (`KismetMathLibrary.MakeRotator` 0.0 0.0 _kinectrotation_z) false false)
  (`self.EnableInput` null)
  (bind _returnvalue (`|CreateWidget` "/Game/Blueprints/Menus/GameOver.GameOver_C"))
  (bind _output_get (set `self.gameOverWidget` _returnvalue))
  (`UserWidget.AddToViewport` _output_get 0))

(event `self.ReceiveTick`
  (params (DeltaSeconds :type "Float (single-precision)"))
  (bind (_kinectrotation_x _kinectrotation_y _kinectrotation_z) (`KismetMathLibrary.BreakVector` (`self.KinectRotation`)))
  ;[1 1 1] Update the Kinect Poseable Mesh to pull data from current centered body
  (bind (_centeredbody _istracked) (`KinectInterfaceComponent.GetCenteredBody` (`self.KinectInterface`)))
  (if _istracked
    (set `KinectPoseableMeshComponent.TargetBody` _centeredbody (`self.KinectPoseableMesh`))
    ;[1 1 1] Vector from Root to Head
    (bind _returnvalue (`PoseableMeshComponent.GetBoneLocationByName` (`self.KinectPoseableMesh`) "head" "ComponentSpace"))
    (`SceneComponent.K2_SetRelativeLocation` (`self.KinectPoseableMesh`) (- (`SceneComponent.RelativeLocation` (`self.Camera`)) (`KismetMathLibrary.GreaterGreater_VectorRotator` _returnvalue (`KismetMathLibrary.MakeRotator` 0.0 0.0 _kinectrotation_z))) false false)
    (`SceneComponent.K2_AddRelativeLocation` (`self.KinectPoseableMesh`) (`self.HeadOffset`) false false)
    (`KinectInterfaceComponent.SetSmoothingParameters` (`self.KinectInterface`) 0.3 0.0)))

(event `self.Torso.OnComponentBeginOverlap`
  (params (OverlappedComponent :type "PrimitiveComponent Object Reference") (OtherActor :type "Actor Object Reference") (OtherComp :type "PrimitiveComponent Object Reference") (OtherBodyIndex :type Integer) (bFromSweep :type Boolean) (SweepResult :type "HitResult Structure (by ref)"))
  ;[1 1 1] Collision
  (`PrimitiveComponent.SetCollisionEnabled` OtherComp "NoCollision")
  (if (`self.ActorHasTag` OtherActor "Bullet")
    (`self.Hit`)))

(event `self.R_Upper_Arm.OnComponentBeginOverlap`
  (params (OverlappedComponent :type "PrimitiveComponent Object Reference") (OtherActor :type "Actor Object Reference") (OtherComp :type "PrimitiveComponent Object Reference") (OtherBodyIndex :type Integer) (bFromSweep :type Boolean) (SweepResult :type "HitResult Structure (by ref)"))
  ;[1 1 1] Collision
  (if (`self.ActorHasTag` OtherActor "Bullet")
    (if (`self.NotHit`)
      _)))

(event `WaveReset`)

(event `self.R_Lower_Arm.OnComponentBeginOverlap`
  (params (OverlappedComponent :type "PrimitiveComponent Object Reference") (OtherActor :type "Actor Object Reference") (OtherComp :type "PrimitiveComponent Object Reference") (OtherBodyIndex :type Integer) (bFromSweep :type Boolean) (SweepResult :type "HitResult Structure (by ref)"))
  ;[1 1 1] Collision
  (if (`self.ActorHasTag` OtherActor "Bullet")
    (if (`self.NotHit`)
      _)))

(event `self.L_Upper_Arm.OnComponentBeginOverlap`
  (params (OverlappedComponent :type "PrimitiveComponent Object Reference") (OtherActor :type "Actor Object Reference") (OtherComp :type "PrimitiveComponent Object Reference") (OtherBodyIndex :type Integer) (bFromSweep :type Boolean) (SweepResult :type "HitResult Structure (by ref)"))
  ;[1 1 1] Collision
  (if (`self.ActorHasTag` OtherActor "Bullet")
    (if (`self.NotHit`)
      _)))

(event `Hit`
  ;[1 1 1] What happens when the player is hit?
  (`PlayerCameraManager.StartCameraFade` (`GameplayStatics.GetPlayerCameraManager` 0) 0.0 0.7 0.2 (struct :`R` 0.6 :`G` 0.006 :`B` 0.006 :`A` 1.0) false false)
  (set `self.Lives` (- (`self.Lives`) 1)))

(event `self.L_Lower_Arm.OnComponentBeginOverlap`
  (params (OverlappedComponent :type "PrimitiveComponent Object Reference") (OtherActor :type "Actor Object Reference") (OtherComp :type "PrimitiveComponent Object Reference") (OtherBodyIndex :type Integer) (bFromSweep :type Boolean) (SweepResult :type "HitResult Structure (by ref)"))
  ;[1 1 1] Collision
  (if (`self.ActorHasTag` OtherActor "Bullet")
    (if (`self.NotHit`)
      _)))

(event `self.Head.OnComponentBeginOverlap`
  (params (OverlappedComponent :type "PrimitiveComponent Object Reference") (OtherActor :type "Actor Object Reference") (OtherComp :type "PrimitiveComponent Object Reference") (OtherBodyIndex :type Integer) (bFromSweep :type Boolean) (SweepResult :type "HitResult Structure (by ref)"))
  ;[1 1 1] Collision
  (if (`self.ActorHasTag` OtherActor "Bullet")
    (if (`self.NotHit`)
      _)))

(event `self.R_Thigh.OnComponentBeginOverlap`
  (params (OverlappedComponent :type "PrimitiveComponent Object Reference") (OtherActor :type "Actor Object Reference") (OtherComp :type "PrimitiveComponent Object Reference") (OtherBodyIndex :type Integer) (bFromSweep :type Boolean) (SweepResult :type "HitResult Structure (by ref)"))
  ;[1 1 1] Collision
  (if (`self.ActorHasTag` OtherActor "Bullet")
    (if (`self.NotHit`)
      _)))

(event `self.L_Thigh.OnComponentBeginOverlap`
  (params (OverlappedComponent :type "PrimitiveComponent Object Reference") (OtherActor :type "Actor Object Reference") (OtherComp :type "PrimitiveComponent Object Reference") (OtherBodyIndex :type Integer) (bFromSweep :type Boolean) (SweepResult :type "HitResult Structure (by ref)"))
  ;[1 1 1] Collision
  (if (`self.ActorHasTag` OtherActor "Bullet")
    (if (`self.NotHit`)
      _)))

(event `self.TriggerBox.OnComponentBeginOverlap`
  (params (OverlappedComponent :type "PrimitiveComponent Object Reference") (OtherActor :type "Actor Object Reference") (OtherComp :type "PrimitiveComponent Object Reference") (OtherBodyIndex :type Integer) (bFromSweep :type Boolean) (SweepResult :type "HitResult Structure (by ref)"))
  (if (`self.ActorHasTag` OtherActor "Bullet")
    (`PrimitiveComponent.SetCollisionEnabled` OtherComp "NoCollision")
    (set `self.BulletsDodged` (+ (`self.BulletsDodged`) 1))))

(fn `UserConstructionScript`)