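; Skyscraper actor that procedurally scatters a field of skyscrapers at BeginPlay, leaving the grid cell at 0,0 empty.
; It walks a square grid spaced by GridSize, and PlaceSkyscraper fills roughly one cell in three.
; Each building is an instance in one of five differently sized instanced mesh components, with random horizontal jitter and height offset.
; Two sizes are added in local space and three in world space.
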(event EventBeginPlay
  (bind _gridsize (Variables|Default|GetgridSize))
  (bind _grids (Variables|Default|Getgrids))
  (for _index (range (stale _result) _grids)
    (for _index_2 (range (stale _result) _grids)
      (if (not (and (== _index 0) (== _index_2 0)))
        (CallFunction|PlaceSkyscraper (* _gridsize _index) (* _index_2 _gridsize))))))

(event Collision|EventActorBeginOverlap
  (params (OtherActor :type Actor%20Object%20Reference)))

(event EventTick
  (params (DeltaSeconds :type Float%20%28single-precision%29)))

(fn ConstructionScript)

(fn PlaceSkyscraper
  (params (x :type Integer) (y :type Integer))
  (bind _returnvalue (Math|Random|RandomIntegerinRange -2000 1000))
  (bind _returnvalue_2 (Math|Random|RandomIntegerinRange -500 500))
  (bind _returnvalue_3 (Math|Random|RandomIntegerinRange -500 500))
  (bind _returnvalue_4 (Math|Conversions|ToFloat(Integer) _returnvalue))
  (bind _returnvalue_5 (+ y _returnvalue_2))
  (bind _returnvalue_6 (+ x _returnvalue_3))
  (bind _returnvalue_7 (Math|Conversions|ToFloat(Integer) _returnvalue_6))
  (bind _returnvalue_8 (Math|Conversions|ToFloat(Integer) _returnvalue_5))
  (bind _returnvalue_9 (Math|Vector|MakeVector _returnvalue_7 _returnvalue_8 _returnvalue_4))
  (bind _returnvalue_10 (Math|Conversions|ToTransform(Vector) _returnvalue_9))
  (if (== 1 (Math|Random|RandomInteger 3))
    (switch int (Math|Random|RandomInteger 5)
      (:0
        (Class|InstancedStaticMeshComponent|AddInstanceWorldSpace (Variables|Default|Get40x40x80) _returnvalue_10))
      (:1
        (Components|InstancedStaticMesh|AddInstance (Variables|Default|Get10x20x40) _returnvalue_10))
      (:2
        (Components|InstancedStaticMesh|AddInstance (Variables|Default|Get20x20x40) _returnvalue_10))
      (:3
        (Class|InstancedStaticMeshComponent|AddInstanceWorldSpace (Variables|Default|Get30x20x40) _returnvalue_10))
      (:4
        (Class|InstancedStaticMeshComponent|AddInstanceWorldSpace (Variables|Default|Get20x10x40) _returnvalue_10)))))